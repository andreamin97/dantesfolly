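; Dante player character Blueprint with camera-relative movement, jump, sword attack, block, dodge roll and interact input.
; Input sets state flags, with attack and block suspending movement while held.
; Custom events toggle the sword hitbox, whose DoOnce-gated overlap applies damage and radial force once per enable.
; Roll picks a forward, backward or sideways impulse from movement input, while CameraRotateY alone drives spring arm and mesh rotation.
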(event OnComponentBeginOverlap(Sword_hitbox)
  (params (OverlappedComponent :type Primitive%20Component%20Object%20Reference) (OtherActor :type Actor%20Object%20Reference) (OtherComp :type Primitive%20Component%20Object%20Reference) (OtherBodyIndex :type Integer) (bFromSweep :type Boolean) (SweepResult :type Hit%20Result%20Structure%20%28by%20ref%29))
  ;[1 1 1] Damage
  (if (!= OtherComp (Game|GetPlayerController 0))
    (Utilities|FlowControl|DoOnce false
      (:Completed
        (Game|Damage|ApplyDamage OtherActor 1e+01 0 0)
        (Physics|AddRadialForce OtherComp (.ImpactPoint (Collision|BreakHitResult SweepResult)) 5e+01 1e+01 "RIF_Constant" false)))))

(event Custom|enable_sword
  ;[1 1 1] Damage
  (Collision|SetCollisionEnabled (Variables|Default|GetSword_hitbox) "QueryAndPhysics")
  (CallFunction|ResetDamage))

(event Custom|disable_sword
  ;[1 1 1] Damage
  (Collision|SetCollisionEnabled (Variables|Default|GetSword_hitbox) "NoCollision"))

(event Custom|Reset%20Damage
  ;[1 1 1] Damage
  (Utilities|FlowControl|DoOnce false) ; enters at Reset
)

(event EventBeginPlay
  (Variables|/Script/Engine.PlayerController|SetbShowMouseCursor (Game|GetPlayerController 0) false)
  (Transformation|SetActorRotation "0,180.000000, 0"))

(event Collision|EventActorBeginOverlap
  (params (OtherActor :type Actor%20Object%20Reference)))

(event EventTick
  (params (DeltaSeconds :type Float%20%28single-precision%29))
  (if (Variables|Default|GetcanMove)
    (Variables|Default|SetForward (Input|AxisValues|GetMoveForward))
    (Variables|Default|SetRight (Input|AxisValues|GetMoveRight))))

(event Input|ActionEvents|InputActionJump
  (params (Key :type Key%20Structure))
  ;[1 1 1] movement
  (:Pressed
    (Character|Jump)
    (Variables|Default|SetisJumping true))
  (:Released
    (Character|StopJumping)))

(event Input|ActionEvents|InputActionAttack
  (params (Key :type Key%20Structure))
  ;[1 1 1] Attack
  (:Pressed
    (Variables|Default|SetisAttacking true)
    (Variables|Default|SetcanMove false))
  (:Released
    (Variables|Default|SetisAttacking false)
    (Variables|Default|SetcanMove true)))

(event Input|ActionEvents|InputActionRoll
  (params (Key :type Key%20Structure))
  ;[1 1 1] Roll
  (:Pressed
    (if (not (AI|Components|NavMovement|IsFalling (Variables|Character|GetCharacterMovement)))
      (Variables|Default|SetisRolling true)
      (Utilities|FlowControl|DoOnce false :!label _label
        (:Completed
          (if (== (Variables|Default|GetRight) 0.0)
            (switch int (Math|Float|Truncate (Variables|Default|GetForward))
              (:Default
                (|DashBackwards :!label _label_2))
              (:0
                (goto _label_2))
              (:1
                (|DashForward)))
            (else
              (|DodgeSideways)))
          (Variables|Default|SetisRolling false)
          (goto _label Reset))))))

(event Input|ActionEvents|InputActionBlock
  (params (Key :type Key%20Structure))
  ;[1 1 1] Block
  (:Pressed
    (Variables|Default|SetisBlocking true)
    (Variables|Default|SetcanMove false))
  (:Released
    (Variables|Default|SetisBlocking false)
    (Variables|Default|SetcanMove true)))

(event Input|ActionEvents|InputActionInteract
  (params (Key :type Key%20Structure))
  (:Pressed
    (Variables|Default|SetInteracting true))
  (:Released
    (Variables|Default|SetInteracting false)))

(event Input|AxisEvents|InputAxisMoveForward
  (params (AxisValue :type Float%20%28single-precision%29))
  ;[1 1 1] movement
  (if (Variables|Default|GetcanMove)
    (Pawn|Input|AddMovementInput (Math|Vector|GetForwardVector (Variables|Default|GetCamera)) (* AxisValue (Variables|Default|GetmovementSpeed)) false)))

(event Input|AxisEvents|InputAxisMoveRight
  (params (AxisValue :type Float%20%28single-precision%29))
  ;[1 1 1] movement
  (if (Variables|Default|GetcanMove)
    (Pawn|Input|AddMovementInput (Math|Vector|GetRightVector (Variables|Default|GetCamera)) (* (Variables|Default|GetmovementSpeed) AxisValue) false)))

(event Input|AxisEvents|InputAxisCameraRotateX
  (params (AxisValue :type Float%20%28single-precision%29))
  ;[1 1 1] Camera rotation
)

(event Input|AxisEvents|InputAxisCameraRotateY
  (params (AxisValue :type Float%20%28single-precision%29))
  ;[1 1 1] Camera rotation
  (CallFunction|RotateCharacter (stale Input|AxisEvents|InputAxisCameraRotateX AxisValue) AxisValue))

(fn ConstructionScript)

(fn TraceUnderMouse
  (bind _returnvalue (Game|GetPlayerController 0))
  (bind _outhit (Collision|LineTraceByChannel (.WorldLocation (Game|Player|ConvertMouseLocationToWorldSpace _returnvalue)) (.location (.HitResult (Game|Player|GetHitResultUnderCursorbyChannel _returnvalue "TraceTypeQuery1" true))) "TraceTypeQuery1" false 0 "ForDuration"))
  (return _outhit))

(fn RotateCharacter
  (params (X :type Float%20%28single-precision%29) (Y :type Float%20%28single-precision%29))
  (bind _camerarotatespeed (Variables|Default|GetcameraRotateSpeed))
  (bind _returnvalue (* X _camerarotatespeed))
  (Transformation|AddRelativeRotation (Variables|Default|GetSpringArm) (Math|Rotator|MakeRotator 0.0 (* Y (Variables|Default|GetcameraRotateSpeed)) _returnvalue) false false)
  (Transformation|AddRelativeRotation (Variables|Character|GetMesh) (Math|Rotator|MakeRotator 0.0 0.0 _returnvalue) false false))