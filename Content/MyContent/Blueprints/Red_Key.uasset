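; Red key pickup actor that the player can loot into the Dante_BP bag.
; A timeline started on BeginPlay drives the cube's yaw.
; Any actor beginning overlap with Collision enables looting and input, as that Dante_BP cast is disconnected; only Dante_BP ending overlap disables them.
; Pressing Interact while lootable adds ItemData to the player pawn's Bag and destroys the key.
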(event OnComponentBeginOverlap(collision)
  (params (OverlappedComponent :type Primitive%20Component%20Object%20Reference) (OtherActor :type Actor%20Object%20Reference) (OtherComp :type Primitive%20Component%20Object%20Reference) (OtherBodyIndex :type Integer) (bFromSweep :type Boolean) (SweepResult :type Hit%20Result%20Structure%20%28by%20ref%29))
  (Variables|Default|SetcanLoot true)
  (Input|EnableInput (Game|GetPlayerController 0)))

(event OnComponentEndOverlap(collision)
  (params (OverlappedComponent :type Primitive%20Component%20Object%20Reference) (OtherActor :type Actor%20Object%20Reference) (OtherComp :type Primitive%20Component%20Object%20Reference) (OtherBodyIndex :type Integer))
  (Utilities|Casting|CastToDante_BP OtherActor)
  (Variables|Default|SetcanLoot false)
  (Input|DisableInput (Game|GetPlayerController 0)))

(event EventBeginPlay
  (bind _rotation (Timeline|Rotation%20and%20bounce Play)
    (:Update
      (Transformation|SetWorldRotation (Variables|Default|GetCube) (Math|Rotator|MakeRotator 0.0 0.0 _rotation) false false))))

(event Collision|EventActorBeginOverlap
  (params (OtherActor :type Actor%20Object%20Reference)))

(event EventTick
  (params (DeltaSeconds :type Float%20%28single-precision%29)))

(event Input|ActionEvents|InputActionInteract
  (params (Key :type Key%20Structure))
  (:Pressed
    (if (Variables|Default|GetcanLoot)
      (bind _asdante_bp (Utilities|Casting|CastToDante_BP (Game|Player|GetPlayerPawn 0)))
      (Utilities|Array|Add (Variables|/Game/MyContent/Dante/Dante_BP.Dante_BP_C|GetBag _asdante_bp) (Variables|Default|GetItemData))
      (Actor|DestroyActor))))

(fn ConstructionScript)