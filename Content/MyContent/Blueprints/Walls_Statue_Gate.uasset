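; Statue gate actor that opens when the player places a matching key from Dante's inventory, then streams in the Lower-city level.
; Box overlap searches Dante_BP's Bag for KeyID, showing either an interact prompt with input enabled or a missing-key message.
; Interact removes the key, reveals the RedKey component, and plays a one-shot timeline that rolls RedGate and calls LoadStreamLevel on each update.
; End overlap hides the prompt only when the Dante cast fails.
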(event OnComponentBeginOverlap(Box)
  (params (OverlappedComponent :type Primitive%20Component%20Object%20Reference) (OtherActor :type Actor%20Object%20Reference) (OtherComp :type Primitive%20Component%20Object%20Reference) (OtherBodyIndex :type Integer) (bFromSweep :type Boolean) (SweepResult :type Hit%20Result%20Structure%20%28by%20ref%29))
  (bind _textrender (Variables|Default|GetTextRender))
  (bind _textrender_2 (Variables|Default|GetTextRender))
  (bind _asdante_bp (Utilities|Casting|CastToDante_BP OtherActor))
  (bind _hasbag (CallFunction|HasKey (Variables|/Game/MyContent/Dante/Dante_BP.Dante_BP_C|GetBag _asdante_bp)))
  (if _hasbag
    (Variables|Default|SetCanPlaceRedKey _hasbag)
    (bind _output_get (Variables|Default|Settag%20text "PressF"))
    (Rendering|Components|TextRender|SetText _textrender_2 _output_get)
    (Rendering|SetVisibility _textrender_2 true false)
    (Input|EnableInput (Game|GetPlayerController 0))
    (else
      (bind _output_get_2 (Variables|Default|Settag%20text "You don't have the key"))
      (Rendering|Components|TextRender|SetText _textrender _output_get_2)
      (Rendering|SetVisibility _textrender true false))))

(event OnComponentEndOverlap(Box)
  (params (OverlappedComponent :type Primitive%20Component%20Object%20Reference) (OtherActor :type Actor%20Object%20Reference) (OtherComp :type Primitive%20Component%20Object%20Reference) (OtherBodyIndex :type Integer))
  (Utilities|Casting|CastToDante_BP OtherActor
    (:CastFailed
      (Rendering|SetVisibility (Variables|Default|GetTextRender) false false)
      (Variables|Default|SetCanPlaceRedKey false)
      (Input|DisableInput (Game|GetPlayerController 0)))))

(event EventBeginPlay)

(event Collision|EventActorBeginOverlap
  (params (OtherActor :type Actor%20Object%20Reference)))

(event EventTick
  (params (DeltaSeconds :type Float%20%28single-precision%29)))

(event Input|ActionEvents|InputActionInteract
  (params (Key :type Key%20Structure))
  (:Pressed
    (if (Variables|Default|GetCanPlaceRedKey)
      (CallFunction|PlaceRedKey)
      (Utilities|FlowControl|DoOnce false
        (:Completed
          (bind _newtrack_0 (Timeline|Timeline_0 Play)
            (:Update
              (CallFunction|OpenRedGate _newtrack_0)
              (Game|LoadStreamLevel(byName) "Lower-city_level" true))))))))

(fn ConstructionScript)

(fn HasKey
  (params (Bag :type Array%20of%20Bag%20Item%20Entry%20Structures))
  (for (_array_element _array_index) Bag
    (if (== (.Id (Utilities|Struct|BreakBagItemEntry _array_element)) (Variables|Default|GetkeyID))
      (return true _array_index)))
  (return false 0))

(fn OpenRedGate
  (params (new%20rot :type Float%20%28single-precision%29))
  (bind _redgate (Variables|Default|GetRedGate))
  (Transformation|SetWorldRotation _redgate (Math|Rotator|MakeRotator new%20rot 0.0 (.yaw (Transformation|GetWorldRotation _redgate))) false false))

(fn PlaceRedKey
  (bind _asdante_bp (Utilities|Casting|CastToDante_BP (Game|Player|GetPlayerPawn 0)))
  (bind (_hasbag _keyindex) (CallFunction|HasKey (Variables|/Game/MyContent/Dante/Dante_BP.Dante_BP_C|GetBag _asdante_bp)))
  (if _hasbag
    (Utilities|Array|RemoveIndex (Variables|/Game/MyContent/Dante/Dante_BP.Dante_BP_C|GetBag _asdante_bp) _keyindex)
    (Rendering|SetVisibility (Variables|Default|GetRed_Key) true false)))