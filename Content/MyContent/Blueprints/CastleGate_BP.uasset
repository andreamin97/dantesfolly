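; Castle gate actor that the player swings open or closed with the Interact input.
; Box2 overlap with Dante_BP sets CanOpen, which gates the Interact press; every press also prints a debug string.
; Open plays or reverses a timeline based on IsOpen, driving the Gate's relative yaw and flipping IsOpen when finished.
; Tick only casts the player character to Dante_BP, with no further effect.
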(event OnComponentBeginOverlap(Box2)
  (params (OverlappedComponent :type Primitive%20Component%20Object%20Reference) (OtherActor :type Actor%20Object%20Reference) (OtherComp :type Primitive%20Component%20Object%20Reference) (OtherBodyIndex :type Integer) (bFromSweep :type Boolean) (SweepResult :type Hit%20Result%20Structure%20%28by%20ref%29))
  (Utilities|Casting|CastToDante_BP OtherActor)
  (Variables|Default|SetCanOpen true))

(event OnComponentEndOverlap(Box2)
  (params (OverlappedComponent :type Primitive%20Component%20Object%20Reference) (OtherActor :type Actor%20Object%20Reference) (OtherComp :type Primitive%20Component%20Object%20Reference) (OtherBodyIndex :type Integer))
  (Utilities|Casting|CastToDante_BP OtherActor)
  (Variables|Default|SetCanOpen false))

(event Custom|Open
  (if (Variables|Default|GetIsOpen)
    (bind _opengate (Timeline|Timeline_0 Reverse)
      (:Update
        (Transformation|SetRelativeRotation (Variables|Default|GetGate) (Math|Rotator|MakeRotator 0.0 0.0 _opengate) false false))
      (:Finished
        (Variables|Default|SetIsOpen (not (Variables|Default|GetIsOpen)))))
    (else
      (Timeline|Timeline_0 Play))))

(event Collision|EventActorBeginOverlap
  (params (OtherActor :type Actor%20Object%20Reference)))

(event EventTick
  (params (DeltaSeconds :type Float%20%28single-precision%29))
  (Utilities|Casting|CastToDante_BP (Game|GetPlayerCharacter 0)))

(event Input|ActionEvents|InputActionInteract
  (params (Key :type Key%20Structure))
  (:Pressed
    (Development|PrintString "Hello")
    (if (Variables|Default|GetCanOpen)
      (CallFunction|Open))))

(fn ConstructionScript)