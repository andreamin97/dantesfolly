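; BigDoor_BP is a double door that swings open when the Dante_BP character enters its trigger box and closes when that character leaves.
; A timeline drives the yaw of the Left and Right leaves in opposite directions, playing on entry and reversing on exit.
; A second LockDoor trigger clears CanOpen when the character touches it, so the door no longer opens afterward.
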(event OnComponentBeginOverlap(boxcollision)
  (params (OverlappedComponent :type Primitive%20Component%20Object%20Reference) (OtherActor :type Actor%20Object%20Reference) (OtherComp :type Primitive%20Component%20Object%20Reference) (OtherBodyIndex :type Integer) (bFromSweep :type Boolean) (SweepResult :type Hit%20Result%20Structure%20%28by%20ref%29))
  (if (Variables|Default|GetcanOpen)
    (Utilities|Casting|CastToDante_BP OtherActor)
    (bind _door_opening_angle (Timeline|Timeline_0 Play)
      (:Update
        (Transformation|SetRelativeRotation (Variables|Default|Getleft) (Math|Rotator|MakeRotator 0.0 0.0 (* _door_opening_angle -1.0)) false false)
        (Transformation|SetRelativeRotation (Variables|Default|Getright) (Math|Rotator|MakeRotator 0.0 0.0 _door_opening_angle) false false)))))

(event OnComponentEndOverlap(boxcollision)
  (params (OverlappedComponent :type Primitive%20Component%20Object%20Reference) (OtherActor :type Actor%20Object%20Reference) (OtherComp :type Primitive%20Component%20Object%20Reference) (OtherBodyIndex :type Integer))
  (Utilities|Casting|CastToDante_BP OtherActor)
  (bind _door_opening_angle (Timeline|Timeline_0 Reverse)
    (:Update
      (Transformation|SetRelativeRotation (Variables|Default|Getleft) (Math|Rotator|MakeRotator 0.0 0.0 (* _door_opening_angle -1.0)) false false)
      (Transformation|SetRelativeRotation (Variables|Default|Getright) (Math|Rotator|MakeRotator 0.0 0.0 _door_opening_angle) false false))))

(event OnComponentBeginOverlap(lockdoor)
  (params (OverlappedComponent :type Primitive%20Component%20Object%20Reference) (OtherActor :type Actor%20Object%20Reference) (OtherComp :type Primitive%20Component%20Object%20Reference) (OtherBodyIndex :type Integer) (bFromSweep :type Boolean) (SweepResult :type Hit%20Result%20Structure%20%28by%20ref%29))
  (Utilities|Casting|CastToDante_BP OtherActor)
  (Variables|Default|SetcanOpen false))

(event EventBeginPlay)

(event Collision|EventActorBeginOverlap
  (params (OtherActor :type Actor%20Object%20Reference)))

(event EventTick
  (params (DeltaSeconds :type Float%20%28single-precision%29)))

(fn ConstructionScript)