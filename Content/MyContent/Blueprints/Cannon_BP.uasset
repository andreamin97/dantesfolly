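; Cannon that the player can take over and fire, with a box overlap toggling whether it can be possessed.
; MoveForward and MoveRight pitch and yaw the Arrow component, gated on the player pawn not being this cannon as written.
; While IsPossessed, which is set outside this graph, Space spawns a cannonball at Arrow1 and launches it with a CannonForce impulse along its forward axis, using limited ammo.
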(event OnComponentBeginOverlap(Box)
  (params (OverlappedComponent :type Primitive%20Component%20Object%20Reference) (OtherActor :type Actor%20Object%20Reference) (OtherComp :type Primitive%20Component%20Object%20Reference) (OtherBodyIndex :type Integer) (bFromSweep :type Boolean) (SweepResult :type Hit%20Result%20Structure%20%28by%20ref%29))
  (Variables|Default|SetCanBePossessed true))

(event OnComponentEndOverlap(Box)
  (params (OverlappedComponent :type Primitive%20Component%20Object%20Reference) (OtherActor :type Actor%20Object%20Reference) (OtherComp :type Primitive%20Component%20Object%20Reference) (OtherBodyIndex :type Integer))
  (Variables|Default|SetCanBePossessed false))

(event EventBeginPlay)

(event Collision|EventActorBeginOverlap
  (params (OtherActor :type Actor%20Object%20Reference)))

(event EventTick
  (params (DeltaSeconds :type Float%20%28single-precision%29)))

(event Input|AxisEvents|InputAxisMoveForward
  (params (AxisValue :type Float%20%28single-precision%29))
  (if (not (== (Game|Player|GetPlayerPawn 0) "Cannon_BP"))
    (Transformation|AddRelativeRotation (Variables|Default|GetArrow) (Math|Rotator|MakeRotator 0.0 (* AxisValue 2.0) 0.0) false false)))

(event Input|AxisEvents|InputAxisMoveRight
  (params (AxisValue :type Float%20%28single-precision%29))
  (if (not (== (Game|Player|GetPlayerPawn 0) "Cannon_BP"))
    (Transformation|AddRelativeRotation (Variables|Default|GetArrow) (Math|Rotator|MakeRotator 0.0 0.0 (* AxisValue 2.0)) false false)))

(event Input|KeyboardEvents|SpaceBar
  (params (Key :type Key%20Structure))
  (bind _arrow1 (Variables|Default|GetArrow1))
  (bind _returnvalue (Transformation|GetWorldTransform _arrow1))
  (:Pressed
    (if (Variables|Default|GetIsPossessed)
      (if (> (Variables|Default|GetNumberOfShots) 0)
        (bind _returnvalue_2 (Game|SpawnActorfromClass "/Game/MyContent/Blueprints/Cannonball_Shooting_BP.Cannonball_Shooting_BP_C" (Math|Transform|MakeTransform (.location _returnvalue) (.rotation _returnvalue) "1,1,1") "Undefined" 0 0))
        (Variables|/Game/MyContent/Blueprints/Cannonball_Shooting_BP.Cannonball_Shooting_BP_C|SetIsShooting _returnvalue_2 true)
        (Physics|AddImpulse (Variables|/Game/MyContent/Blueprints/Cannonball_Shooting_BP.Cannonball_Shooting_BP_C|GetSphere _returnvalue_2) (Math|Vector|RotateVector (Math|Vector|MakeVector (Variables|Default|GetCannonForce) 0.0 0.0) (.rotation _returnvalue)) "None" false)
        (Math|Integer|DecrementInt (Variables|Default|GetNumberOfShots))
        (else
          (Development|PrintString "Out of Ammo"))))))

(fn ConstructionScript)