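; Gate actor that the player opens and closes with the Interact input while standing near it.
; Two trigger boxes each show their own text prompt and set a shared CanOpen flag when Dante_BP overlaps.
; Open plays or reverses a timeline that sweeps the gate along absolute world Z, flipping IsOpen when it finishes.
; Tick only casts the player character to Dante_BP and does nothing else.
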(event OnComponentBeginOverlap(Box)
  (params (OverlappedComponent :type Primitive%20Component%20Object%20Reference) (OtherActor :type Actor%20Object%20Reference) (OtherComp :type Primitive%20Component%20Object%20Reference) (OtherBodyIndex :type Integer) (bFromSweep :type Boolean) (SweepResult :type Hit%20Result%20Structure%20%28by%20ref%29))
  (Utilities|Casting|CastToDante_BP OtherActor)
  (Rendering|SetVisibility (Variables|Default|GetTextRender) true false)
  (Variables|Default|SetCanOpen true))

(event OnComponentEndOverlap(Box)
  (params (OverlappedComponent :type Primitive%20Component%20Object%20Reference) (OtherActor :type Actor%20Object%20Reference) (OtherComp :type Primitive%20Component%20Object%20Reference) (OtherBodyIndex :type Integer))
  (Utilities|Casting|CastToDante_BP OtherActor)
  (Rendering|SetVisibility (Variables|Default|GetTextRender) false false)
  (Variables|Default|SetCanOpen false))

(event OnComponentBeginOverlap(Box1)
  (params (OverlappedComponent :type Primitive%20Component%20Object%20Reference) (OtherActor :type Actor%20Object%20Reference) (OtherComp :type Primitive%20Component%20Object%20Reference) (OtherBodyIndex :type Integer) (bFromSweep :type Boolean) (SweepResult :type Hit%20Result%20Structure%20%28by%20ref%29))
  (Utilities|Casting|CastToDante_BP OtherActor)
  (Rendering|SetVisibility (Variables|Default|GetTextRender1) true false)
  (Variables|Default|SetCanOpen true))

(event OnComponentEndOverlap(Box1)
  (params (OverlappedComponent :type Primitive%20Component%20Object%20Reference) (OtherActor :type Actor%20Object%20Reference) (OtherComp :type Primitive%20Component%20Object%20Reference) (OtherBodyIndex :type Integer))
  (Utilities|Casting|CastToDante_BP OtherActor)
  (Rendering|SetVisibility (Variables|Default|GetTextRender1) false false)
  (Variables|Default|SetCanOpen false))

(event Custom|Open
  (bind _gate (Variables|Default|GetGate))
  (bind _returnvalue (Transformation|GetWorldLocation _gate))
  (if (Variables|Default|GetIsOpen)
    (bind _opengate (Timeline|Timeline_0 Reverse)
      (:Update
        (Transformation|SetWorldLocation _gate (Math|Vector|MakeVector (.x _returnvalue) (.y _returnvalue) _opengate) true false))
      (:Finished
        (Variables|Default|SetIsOpen (not (Variables|Default|GetIsOpen)))))
    (else
      (Timeline|Timeline_0 Play))))

(event EventBeginPlay)

(event Collision|EventActorBeginOverlap
  (params (OtherActor :type Actor%20Object%20Reference)))

(event EventTick
  (params (DeltaSeconds :type Float%20%28single-precision%29))
  (Utilities|Casting|CastToDante_BP (Game|GetPlayerCharacter 0)))

(event Input|ActionEvents|InputActionInteract
  (params (Key :type Key%20Structure))
  (:Pressed
    (if (Variables|Default|GetCanOpen)
      (CallFunction|Open))))

(fn ConstructionScript)