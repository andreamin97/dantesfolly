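; Gruntling enemy Blueprint that tracks health and reports whether it perceives the player.
; Health starts at MaxHp on BeginPlay; AnyDamage subtracts from it, destroying the actor at zero or below and otherwise printing the remaining HP.
; AI perception updates for Dante_BP write the sensed state to the CanSeePlayer Blackboard key.
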(event OnTargetPerceptionUpdated(AIPerception)
  (params (Actor :type Actor%20Object%20Reference) (Stimulus :type AI%20Stimulus%20Structure))
  (Utilities|Casting|CastToDante_BP Actor)
  (AI|Components|Blackboard|SetValueasBool (AI|GetBlackboard 0) (Utilities|Name|MakeLiteralName "CanSeePlayer") (.bSuccessfullySensed (Utilities|Struct|BreakAIStimulus Stimulus))))

(event EventBeginPlay
  (Variables|Default|SetCurrentHp (Variables|Default|GetMaxHp)))

(event Collision|EventActorBeginOverlap
  (params (OtherActor :type Actor%20Object%20Reference)))

(event EventTick
  (params (DeltaSeconds :type Float%20%28single-precision%29)))

(event Game|Damage|EventAnyDamage
  (params (Damage :type Float%20%28single-precision%29) (DamageType :type Damage%20Type%20Object%20Reference) (InstigatedBy :type Controller%20Object%20Reference) (DamageCauser :type Actor%20Object%20Reference))
  (bind _output_get (Variables|Default|SetCurrentHp (- (Variables|Default|GetCurrentHp) Damage)))
  (if (<= _output_get 0.0)
    (Actor|DestroyActor)
    (else
      (Development|PrintString (Utilities|String|ToString(Float) _output_get)))))

(fn ConstructionScript)